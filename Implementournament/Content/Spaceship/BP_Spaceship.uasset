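; Player-controlled spaceship with physics-based thrust, steering, boosting and laser fire, driven by Enhanced Input.
; Each tick applies forces with a lerped speed cap, fires all laser weapon components on a cooldown, then updates thruster and space-particle VFX, camera FOV and shakes.
; Steering pushes along world Y/Z, damped by speed and boost, while only the mesh banks cosmetically.
; Empty events expose thrust, speed, steering, boost, collision and shooting changes as hooks.
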(event Custom|OnStoppedShooting
  ;[0.03 0.03 0.03] Shooting Lasers
)

(event Custom|OnShootLasers
  ;[0.03 0.03 0.03] Shooting Lasers
)

(event Custom|OnStoppedBoosting
  ;[0.03 0.03 0.03] Boosting Events
)

(event Custom|OnThrustStateChanged
  (params (isThrustActive :type Boolean))
  ;[0.03 0.03 0.03] Movement Events
)

(event Custom|OnSteerInputChanged
  (params (steerInputX :type Float%20%28double-precision%29) (steerInputY :type Float%20%28double-precision%29))
  ;[0.03 0.03 0.03] Movement Events
)

(event Custom|OnForwardSpeedChanged
  (params (forwardSpeed :type Float%20%28double-precision%29))
  ;[0.03 0.03 0.03] Movement Events
)

(event Custom|OnStartedBoosting
  ;[0.03 0.03 0.03] Boosting Events
)

(event Custom|OnStartedShooting
  ;[0.03 0.03 0.03] Shooting Lasers
)

(event Custom|OnSpaceShipCollided
  (params (collisionForce :type Float%20%28double-precision%29))
  ;[0.03 0.03 0.03] Collision Events
)

(event EventTick
  (params (DeltaSeconds :type Float%20%28single-precision%29))
  ;[0.03 0.03 0.03] Event Tick
  (Utilities|UpdateMovement)
  (Utilities|CheckforBoosting)
  (Utilities|UpdateShootingLasers)
  (Utilities|UpdateCosmetics)
  (Utilities|UpdateCamera)
  (|UpdateLastFrameVariables))

(event EventBeginPlay
  ;[0.03 0.03 0.03] Event Begin Play
  (Utilities|SetupInputMappingContext)
  (Utilities|StartCameraShakeNoise)
  (Utilities|AssignLaserProjectileComponents)
  (Utilities|SetupMaterials)
  (Utilities|StartInitialCameraFade))

(fn ConstructionScript)

(event Input|EnhancedActionEvents|EnhancedInputActionIA_Steer
  (params (ActionValue :type Vector%202D%20Structure) (ElapsedSeconds :type Float%20%28double-precision%29) (TriggeredSeconds :type Float%20%28double-precision%29) (InputAction :type Input%20Action%20Object%20Reference :default "/Game/Input/IA_Steer.IA_Steer"))
  (:Triggered
    (Variables|Input|SetsteerInputX (.x ActionValue) :!label _label)
    (Variables|Input|SetsteerInputY (Math|Float|SelectFloat (* (.y ActionValue) -1.0) (.y ActionValue) (Variables|Movement|GetShouldInvertYMovement)))
    (Utilities|FlowControl|Sequence
      (:then_0
        (if (|GetHasSteerInputChanged)
          (CallFunction|OnSteerInputChanged (Variables|Input|GetsteerInputX) (Variables|Input|GetsteerInputY))))
      (:then_1
        (Variables|Input|SetsteerInputXLastFrame (Variables|Input|GetsteerInputX))
        (Variables|Input|SetsteerInputYLastFrame (Variables|Input|GetsteerInputY)))))
  (:Started
    (goto _label))
  (:Completed
    (goto _label)))

(event Input|EnhancedActionEvents|EnhancedInputActionIA_Thrust
  (params (ActionValue :type Float%20%28double-precision%29) (ElapsedSeconds :type Float%20%28double-precision%29) (TriggeredSeconds :type Float%20%28double-precision%29) (InputAction :type Input%20Action%20Object%20Reference :default "/Game/Input/IA_Thrust.IA_Thrust"))
  (:Triggered
    (Variables|Input|SetthrustInput ActionValue :!label _label))
  (:Started
    (goto _label))
  (:Completed
    (goto _label)))

(event Input|EnhancedActionEvents|EnhancedInputActionIA_Boost
  (params (ActionValue :type Boolean) (ElapsedSeconds :type Float%20%28double-precision%29) (TriggeredSeconds :type Float%20%28double-precision%29) (InputAction :type Input%20Action%20Object%20Reference :default "/Game/Input/IA_Boost.IA_Boost"))
  (:Started
    (Variables|Input|SetboostInput ActionValue :!label _label))
  (:Completed
    (goto _label)))

(event Input|EnhancedActionEvents|EnhancedInputActionIA_Shoot
  (params (ActionValue :type Boolean) (ElapsedSeconds :type Float%20%28double-precision%29) (TriggeredSeconds :type Float%20%28double-precision%29) (InputAction :type Input%20Action%20Object%20Reference :default "/Game/Input/IA_Shoot.IA_Shoot"))
  (:Started
    (Variables|Input|SetshootInput ActionValue)
    (CallFunction|OnStartedShooting))
  (:Completed
    (Variables|Input|SetshootInput ActionValue)
    (CallFunction|OnStoppedShooting)))

(event Input|EnhancedActionEvents|EnhancedInputActionIA_Exit
  (params (ActionValue :type Float%20%28double-precision%29) (ElapsedSeconds :type Float%20%28double-precision%29) (TriggeredSeconds :type Float%20%28double-precision%29) (InputAction :type Input%20Action%20Object%20Reference :default "/Game/Input/IA_Exit.IA_Exit"))
  (Game|QuitGame 0 "Quit" false))

(event Collision|EventHit
  (params (MyComp :type Primitive%20Component%20Object%20Reference) (Other :type Actor%20Object%20Reference) (OtherComp :type Primitive%20Component%20Object%20Reference) (bSelfMoved :type Boolean) (HitLocation :type Vector :default "0, 0, 0") (HitNormal :type Vector :default "0, 0, 0") (NormalImpulse :type Vector :default "0, 0, 0") (Hit :type Hit%20Result%20Structure%20%28by%20ref%29))
  ;[0.03 0.03 0.03] Check for min collision force
  (if (> (Math|Vector|VectorLength NormalImpulse) (Variables|Collisions|GetMinCollisionForceForEvents))
    ;[0.03 0.03 0.03] Check for min delay between impacts
    (if (> (Utilities|Time|GetGameTimeinSeconds) (+ (Variables|Collisions|GettimeLastCollided) (Variables|Collisions|GetMinDurationBetweenCollisionEvents)))
      (CallFunction|OnSpaceShipCollided (Math|Vector|VectorLength NormalImpulse))
      (Variables|Collisions|SettimeLastCollided (Utilities|Time|GetGameTimeinSeconds)))))